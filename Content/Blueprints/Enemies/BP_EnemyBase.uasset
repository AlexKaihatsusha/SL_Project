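; Base sword-wielding enemy character for AI control, with health, patrol route and movement-speed accessors.
; It spawns a sheathed sword on BeginPlay, moves it to the hand socket when equipping, and plays montages that signal equip and attack end, even if interrupted.
; Health, healing and damage delegate to ACDamageSystem, whose OnDeath is bound in the Construction Script.
; Death unpossesses the AI controller, ragdolls the mesh and drops the sword, both on timed lifespans.
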(event Custom|SpawnSword
  (bind _returnvalue (Game|SpawnActorfromClass "/Game/Blueprints/DamageActors/Sword/BP_BaseSword.BP_BaseSword_C" (Transformation|GetActorTransform) "Undefined" "MultiplyWithRoot" 0 self))
  (bind _output_get (Variables|Default|SetSwordRef _returnvalue))
  (Transformation|AttachComponentToComponent _output_get (Variables|Character|GetMesh) "sword_pocket" "SnapToTarget" "SnapToTarget" "SnapToTarget" true)
  (Variables|Default|SetIsWeaponEquipped false))

(event Custom|Death
  (bind _mesh (Variables|Character|GetMesh))
  (Variables|Default|SetIsDead true)
  (bind _asaic_enemy_base (Utilities|Casting|CastToAIC_EnemyBase (AI|GetAIController self)))
  (Pawn|UnPossess _asaic_enemy_base)
  (Physics|SetSimulatePhysics _mesh true)
  (Collision|SetCollisionEnabled _mesh "QueryAndPhysics")
  (Actor|SetLifeSpan 1e+01)
  (bind _swordref (Variables|Default|GetSwordRef)
    (:then
      (Transformation|DetachFromComponent (Variables|/Script/Engine.Actor|GetRootComponent _swordref) "KeepRelative" "KeepRelative" "KeepRelative" true)
      (Physics|SetSimulatePhysics (Variables|/Game/Blueprints/DamageActors/Sword/BP_BaseSword.BP_BaseSword_C|GetStaticMesh _swordref) true)
      (Actor|SetLifeSpan _swordref 1e+01))
    (:else)))

(event Custom|EquipWeapon
  (CallFunction|AttachSwordtoHand)
  (Animation|Montage|PlayMontage (Variables|Character|GetMesh) "/Game/Assets/PlayerAnimations/Animations/Sword/AM_Draw_Sword.AM_Draw_Sword" 0.8
    (:OnCompleted
      _)
    (:OnInterrupted
      _))
  (Variables|Default|SetIsEquipping false)
  (Variables|Default|SetIsWeaponEquipped true)
  (Default|CallOnWeaponEquip))

(event Custom|Attack
  (Animation|Montage|PlayMontage (Variables|Character|GetMesh) "/Game/Assets/PlayerAnimations/Animations/Sword/AM_Sword_And_Shield_Slash.AM_Sword_And_Shield_Slash"
    (:OnCompleted
      _)
    (:OnInterrupted
      _))
  (Default|CallOnAttackEnd))

(event EventBeginPlay
  (CallFunction|SpawnSword))

(fn ConstructionScript
  (EventDispatchers|BindEventtoOnDeath (Variables|Default|GetAC_DamageSystem) (EventDispatchers|CreateEvent :!event Custom|Death)))

(fn AttachSwordtoHand
  (if (not (Variables|Default|GetIsEquipping))
    (bind _swordref (Variables|Default|GetSwordRef)
      (:then
        (Transformation|DetachFromComponent (Variables|/Script/Engine.Actor|GetRootComponent _swordref) "KeepWorld" "KeepWorld" "KeepWorld" true)
        (bind _returnvalue (Transformation|AttachComponentToComponent _swordref (Variables|Character|GetMesh) "hand_r_sword_socket" "SnapToTarget" "SnapToTarget" "SnapToTarget" true))
        (Variables|Default|SetIsEquipping _returnvalue))
      (:else))))

(fn GetCurrentHealth
  (bind _returnvalue (Class|DamageSystem|GetCurrentHealth (Variables|Default|GetAC_DamageSystem)))
  (return _returnvalue))

(fn GetMaxHealth
  (bind _returnvalue (Class|DamageSystem|GetMaxHealth (Variables|Default|GetAC_DamageSystem)))
  (return _returnvalue))

(fn GetPatrolRoute
  (return (Variables|Default|GetPatrolRoute)))

(fn Heal
  (params (HealAmount :type Float%20%28single-precision%29))
  (bind _returnvalue (Class|DamageSystem|Heal (Variables|Default|GetAC_DamageSystem) HealAmount))
  (return _returnvalue))

(fn SetMovementSpeed
  (params (SpeedMode :type E_MovementSpeedModes%20Enum :default "NewEnumerator0"))
  (bind _output_get (Variables|/Script/Engine.CharacterMovementComponent|SetMaxWalkSpeed (Variables|Character|GetCharacterMovement) (Utilities|Select :Index SpeedMode :NewEnumerator0 0.0 :NewEnumerator1 1e+02 :NewEnumerator5 2.5e+02 :NewEnumerator2 5e+02)))
  (return _output_get))

(fn TakeDamage
  (params (DamageData :type Damage%20Data%20Structure))
  (bind _returnvalue (Class|DamageSystem|TakeDamage (Variables|Default|GetAC_DamageSystem) DamageData))
  (return _returnvalue))