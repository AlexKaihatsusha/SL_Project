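; BP_PatrolRoute is a placeable patrol path for enemies, built on a PatrolRoute spline.
; GetSplinePointAsWorldPosition returns the world location of the spline point at CurrentIndex.
; IncrementControlRoute steps CurrentIndex by Direction, flipping Direction at the first and last points so the route is walked back and forth rather than looped.
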(event Custom|IncrementControlRoute
  ;[0 0 0 0.5] Move Index through the spline points in forward/back directions, depends on Direction value with ranges [-1,1]
  (bind _output_get (Variables|Default|SetCurrentIndex (+ (Variables|Default|GetCurrentIndex) (Variables|Default|GetDirection))))
  (if (== _output_get (- (Spline|GetNumberOfSplinePoints (Variables|Default|GetPatrolRoute)) 1))
    (Variables|Default|SetDirection -1)
    (elif (== (Variables|Default|GetCurrentIndex) 0)
      (Variables|Default|SetDirection 1))))

(event EventBeginPlay)

(event Collision|EventActorBeginOverlap
  (params (OtherActor :type Actor%20Object%20Reference)))

(event EventTick
  (params (DeltaSeconds :type Float%20%28single-precision%29)))

(fn ConstructionScript)

(fn GetSplinePointasWorldPosition
  (return (Spline|GetLocationatSplinePoint (Variables|Default|GetPatrolRoute) (Variables|Default|GetCurrentIndex) "World")))