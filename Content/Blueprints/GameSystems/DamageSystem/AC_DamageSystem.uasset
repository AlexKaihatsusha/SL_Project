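; AC_DamageSystem is a damage component that resolves incoming hits for its owner.
; TakeDamage overrides a parent function and uses CanBeDamaged to branch into blocked, damaged or no damage, based on death, invincibility and blocking, plus the hit's flags.
; Blocks broadcast OnBlocked with parry eligibility, while damage triggers OnDeath or, if interruptible or forced, OnDamageResponse with the response type.
; Every outcome records whether damage landed and returns the parent's debug-only result.
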(event EventBeginPlay)

(event EventTick
  (params (DeltaSeconds :type Float%20%28single-precision%29)))

(fn TakeDamage
  (params (DamageData :type Damage%20Data%20Structure))
  (bind (_amount _bheadshot _damagetype _responsedamagetype _bforceanimationinterrupt _bdoinvincibledamage _bcanbeblocked _bcanbeparried) (Utilities|Struct|BreakDamageData DamageData))
  (bind _returnvalue (Class|DamageSystem|IsOwnerDead))
  (Utilities|CanbeDamaged _bdoinvincibledamage _bcanbeblocked
    (:BlockDamage
      (Development|PrintString "Damage Is blocked")
      (Default|CallOnBlocked _bcanbeparried)
      (Variables|Default|SetIsDamageReceived false)
      ;[0 0 0 0.5] Parent Implementation just has a debug logic
      (bind _returnvalue_2 (|CallParentFunction DamageData))
      (return _returnvalue_2))
    (:DoDamage
      (Development|PrintString "Do Damage" true true "(R=1.000000,G=0.000000,B=0.729800,A=1.000000)")
      (Class|DamageSystem|ApplyDamage _amount)
      (if _returnvalue
        ;[0 0 0 0.5] OnDeath
        (Variables|Default|SetIsDead _returnvalue)
        (Default|CallOnDeath)
        (elif (or (Variables|Default|GetIsInterruptible) _bforceanimationinterrupt)
          (Development|PrintString (Utilities|String|EnumtoString _responsedamagetype))
          (Default|CallOnDamageResponse _responsedamagetype)))
      (Variables|Default|SetIsDamageReceived true)
      ;[0 0 0 0.5] Parent Implementation just has a debug logic
      (bind _returnvalue_3 (|CallParentFunction DamageData))
      (return _returnvalue_3))
    (:NoDamage
      (Development|PrintString "No Damage")
      (Variables|Default|SetIsDamageReceived false)
      ;[0 0 0 0.5] Parent Implementation just has a debug logic
      (bind _returnvalue_4 (|CallParentFunction DamageData))
      (return _returnvalue_4))))