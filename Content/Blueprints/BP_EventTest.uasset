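; BP_EventTest is a test event with begin, update, end and IsDone hooks that turns the level's enemies hostile toward the player.
; OnBegin caches all BP_EnemyBase actors and starts a short timer, or finishes immediately if none exist.
; When the timer fires, each enemy's AIC_EnemyBase controller is set to attacking player 0's character, setting the Finished flag that IsDone reports.
; Debug prints trace each stage.
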(event Custom|Timer%20is%20finished
  (bind _enemyrefs (Variables|Default|GetEnemyRefs))
  ;[0 0 0 0.5] Get all enemies, and set Attacking state after 3 seconds
  (if (Utilities|Array|IsNotEmpty _enemyrefs)
    (for _array_element _enemyrefs
      (bind _asbp_enemy_base (Utilities|Casting|CastToBP_EnemyBase _array_element))
      (bind _asaic_enemy_base (Utilities|Casting|CastToAIC_EnemyBase (AI|GetAIController _asbp_enemy_base)))
      (Default|SetStateasAttacking _asaic_enemy_base (Game|GetPlayerCharacter 0))
      (Variables|Default|SetFinished true))
    (else
      (Development|PrintString "Array Is EMPTY" false true "(R=1.000000,G=0.000000,B=0.057255,A=1.000000)")
      (Variables|Default|SetFinished true))))

(event EventOnEnd
  (Development|PrintString self "OnEnd" true true "(R=0.011136,G=1.000000,B=0.000000,A=1.000000)"))

(event EventOnBegin
  (params (bFirstTime :type Boolean))
  (Development|PrintString self "Started" true true "(R=0.020501,G=0.066947,B=1.000000,A=1.000000)")
  (Utilities|IsValid (Class|GameEventBehaviour|GetWorld)
    (:Is%20Valid
      (bind _outactors (Actor|GetAllActorsOfClass "/Game/Blueprints/Enemies/BP_EnemyBase.BP_EnemyBase_C"))
      (bind _output_get (Variables|Default|SetEnemyRefs _outactors))
      (if (Utilities|Array|IsEmpty _output_get)
        (Development|PrintString "Array Is EMPTY" true true "(R=1.000000,G=0.000000,B=0.057255,A=1.000000)")
        (Variables|Default|SetFinished true)
        (else
          (bind _returnvalue (Utilities|Time|SetTimerbyEvent (delegate Custom|Timer%20is%20finished) 2.0))
          (Variables|Default|SetTestTimer _returnvalue))))))

(event EventOnUpdate
  (Development|PrintString self "Running" true true "(R=1.000000,G=0.093227,B=0.000000,A=1.000000)" 0.0))

(fn IsDone
  (return (Variables|Default|GetFinished)))

(fn ConstructionScript)