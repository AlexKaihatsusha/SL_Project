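; Bow arrow projectile that stays inert until Fire adds a projectile movement component, with draw Strength scaling speed, gravity and damage.
; On a blocking hit it sticks to the struck bone with impact effects, pushes physics bodies and expires, while arrow-on-arrow hits destroy both.
; Damageable targets receive damage adjusted by physical surface (head boosted, hands and feet reduced), with a color-coded damage number widget.
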(event OnComponentHit(CollisionBox)
  (params (HitComponent :type Primitive%20Component%20Object%20Reference) (OtherActor :type Actor%20Object%20Reference) (OtherComp :type Primitive%20Component%20Object%20Reference) (NormalImpulse :type Vector :default "0, 0, 0") (Hit :type Hit%20Result%20Structure%20%28by%20ref%29))
  (bind (_bblockinghit _binitialoverlap _time _distance _location _impactpoint _normal _impactnormal _physmat _hitactor _hitcomponent _hitbonename) (Collision|BreakHitResult Hit))
  (if _bblockinghit
    (Utilities|FlowControl|Sequence
      (:then_0
        (Development|SetHiddeninGame (Variables|Default|GetNiagara_Trail) true false)
        (bind _projectilemovementcomponent (Variables|Default|GetProjectileMovementComponent)
          (:then
            (Development|PrintString (Utilities|String|ToString(Name) _hitbonename))
            (Components|DestroyComponent _projectilemovementcomponent)
            (Collision|SetCollisionEnabled (Variables|Default|GetCollisionBox) "NoCollision")
            (if (!= (Utilities|GetClass _hitactor) "BP_Arrow_C")
              (Transformation|SetActorLocation (+ (Transformation|GetActorLocation) (* (Transformation|GetActorForwardVector) 35.0)) false false)
              (Transformation|AttachComponentToComponent _hitcomponent _hitbonename "KeepWorld" "KeepWorld" "KeepWorld" true)
              (Audio|PlaySoundatLocation "/Game/Assets/SFX/Bow/arrow-impact-1.arrow-impact-1" (Transformation|GetActorLocation) "0, 0, 0" 1.0 1.0 0.0 0 0 0 0)
              (Actor|SetLifeSpan 5.0)
              (Niagara|SpawnSystematLocation (Variables|Default|GetImpactEffectSystem) _location (Math|Conversions|RotationFromXVector (- (Transformation|GetActorForwardVector) "")))
              ;[0 0 0 0.5] Apply Impulse if target is Simulating physics
              (if (Physics|IsSimulatingPhysics _hitcomponent "None")
                (Physics|AddImpulse _hitcomponent (Variables|Default|GetArrowVelocity) _hitbonename true))
              (else
                ;[0 0 0 0.5] Destoy both arrows if overlap with each other
                (Actor|DestroyActor _hitactor)
                (Actor|DestroyActor))))
          (:else)))
      (:then_1
        (if (Utilities|DoesObjectImplementInterface _hitactor "/Script/SoloLeveling.Damageable")
          (bind _returnvalue (UserInterface|CreateWidget "/Game/Blueprints/Widgets/WBP_DamageNumber.WBP_DamageNumber_C" (Game|GetPlayerController 0)))
          (Variables|Default|SetWidgetNumber _returnvalue)
          (switch Utilities|FlowControl|Switch|SwitchonEPhysicalSurface (Variables|/Script/PhysicsCore.PhysicalMaterial|GetSurfaceType _physmat)
            (:SurfaceType_Default
              ;[0 0 0 0.5] Set Damage Number, and add to viewport the widget
              (Default|SetDamage (Variables|Default|GetWidgetNumber) (Math|Float|Truncate (.amount (Variables|Default|GetDamageData))) (Utilities|Struct|MakeSlateColor "(R=0.131427,G=0.198641,B=1.000000,A=1.000000)" "UseColor_Specified") :!label _label))
            (:SurfaceType1
              ;[0 0 0 0.5] HEADSHOOOOOOOOT
              (Variables|Default|SetDamageData (Utilities|Struct|MakeDamageData (* (.amount (Variables|Default|GetDamageData)) (Variables|Default|GetHeadshotDamageMultiplier)) true (.damagetype (Variables|Default|GetDamageData)) (.responsedamagetype (Variables|Default|GetDamageData)) false false false false))
              (Default|SetDamage (Variables|Default|GetWidgetNumber) (Math|Float|Truncate (.amount (Variables|Default|GetDamageData))) (Utilities|Struct|MakeSlateColor "(R=1.000000,G=0.350744,B=0.073683,A=1.000000)" "UseColor_Specified")))
            (:SurfaceType2
              (goto _label))
            (:SurfaceType3
              ;[0 0 0 0.5] Divide damage if foot or hand
              (Variables|Default|SetDamageData (Utilities|Struct|MakeDamageData (/ (.amount (Variables|Default|GetDamageData)) (Variables|Default|GetHeadshotDamageMultiplier)) false (.damagetype (Variables|Default|GetDamageData)) (.responsedamagetype (Variables|Default|GetDamageData)) false false false false) :!label _label_2)
              (Default|SetDamage (Variables|Default|GetWidgetNumber) (Math|Float|Truncate (.amount (Variables|Default|GetDamageData))) (Utilities|Struct|MakeSlateColor "(R=0.951217,G=1.000000,B=0.878522,A=1.000000)" "UseColor_Specified")))
            (:SurfaceType4
              (goto _label_2)))
          (bind _returnvalue_2 (Class|Damageable|TakeDamage(Message) _hitactor (Variables|Default|GetDamageData)))
          (if _returnvalue_2
            (UserInterface|Viewport|AddtoViewport (Variables|Default|GetWidgetNumber) -1)
            (Class|Widget|SetRenderTranslation (Variables|Default|GetWidgetNumber) (Math|Vector2D|MakeVector2D (+ (.x (.translation (Variables|/Script/UMG.Widget|GetRenderTransform (Variables|Default|GetWidgetNumber)))) (Math|Random|RandomFloatinRange -1e+01 1e+01)) (+ (.y (.translation (Variables|/Script/UMG.Widget|GetRenderTransform (Variables|Default|GetWidgetNumber)))) (Math|Random|RandomFloatinRange -1e+01 1e+01))))))))))

(event Custom|Fire
  (params (Direction :type Vector) (PossibleHitLocation :type Vector) (Strength :type Float%20%28double-precision%29))
  (bind _returnvalue (AddComponent|AddProjectileMovementComponent))
  ;[0 0 0 0.5] rotate to hit point
  (bind _output_get (Variables|Default|SetFireLocation (Transformation|GetActorLocation)))
  (Transformation|SetActorRotation (Math|Rotator|MakeRotfromX (- (Math|Vector|Normalize PossibleHitLocation) _output_get)))
  (Variables|Default|SetProjectileMovementComponent _returnvalue)
  (bind _output_get_2 (Variables|/Script/Engine.MovementComponent|SetVelocity _returnvalue (* Direction (Math|Float|Lerp (Variables|Default|GetMinSpeed) (Variables|Default|GetMaxSpeed) Strength))))
  (Variables|Default|SetArrowVelocity _output_get_2)
  (Variables|/Script/Engine.ProjectileMovementComponent|SetProjectileGravityScale _returnvalue (Math|Float|Lerp (Variables|Default|GetMaxGravity) (Variables|Default|GetMinGravity) Strength))
  (Variables|Default|SetDamageData (Utilities|Struct|MakeDamageData (Math|Float|Lerp 1e+01 (.amount (Variables|Default|GetDamageData)) Strength) (.bheadshot (Variables|Default|GetDamageData)) (.damagetype (Variables|Default|GetDamageData)) (.responsedamagetype (Variables|Default|GetDamageData)) false false false false))
  (Audio|PlaySoundatLocation (Variables|Default|GetWhoshSound) (Transformation|GetActorLocation) "0, 0, 0" 1.0 1.0 0.4 0 0 0 0)
  (Development|SetHiddeninGame (Variables|Default|GetNiagara_Trail) false false)
  (Collision|SetCollisionEnabled (Variables|Default|GetCollisionBox) "QueryAndPhysics"))

(event EventBeginPlay
  ;[0 0 0 0.5] Hide the Trail
  (Development|SetHiddeninGame (Variables|Default|GetNiagara_Trail) true false)
  (Collision|SetCollisionEnabled (Variables|Default|GetCollisionBox) "NoCollision"))

(event Collision|EventActorBeginOverlap
  (params (OtherActor :type Actor%20Object%20Reference)))

(event EventTick
  (params (DeltaSeconds :type Float%20%28single-precision%29)))

(fn ConstructionScript)