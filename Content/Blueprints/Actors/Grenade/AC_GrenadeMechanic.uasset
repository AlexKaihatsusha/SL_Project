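; Actor component that lets its owning Character hold and throw a BP_HealthGrenade.
; CreateGrenade spawns a scaled-down grenade with physics off, attaches it to the hand_r socket and stores the attach result in IsThrowing to block repeat spawns.
; ThrowGrenade detaches it, enables physics, launches it via UseGrenage along the camera's forward vector and clears the reference.
; IsThrowing resets only on BeginPlay here, not after a throw.
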(event Custom|CreateGrenade
  (CallFunction|SpawnGrenade))

(event Custom|ThrowGrenade
  (params (FollowCamera :type Camera%20Component%20Object%20Reference))
  (CallFunction|UseGrenade FollowCamera))

(event EventBeginPlay
  ;[0 0 0 0.5] BeginPlay set Character Ref
  (bind _ascharacter (Utilities|Casting|CastToCharacter (Components|GetOwner)))
  (Variables|Default|SetCharacterRef _ascharacter)
  (Variables|Default|SetIsThrowing false))

(event EventTick
  (params (DeltaSeconds :type Float%20%28single-precision%29)))

(fn SpawnGrenade
  (bind _characterref (Variables|Default|GetCharacterRef))
  (if (not (Variables|Default|GetIsThrowing))
    (bind _returnvalue (Game|SpawnActorfromClass "/Game/Blueprints/Actors/Grenade/BP_HealthGrenade.BP_HealthGrenade_C" (Math|Transform|MakeTransform "0, 0, 0" "0, 0, 0" "0.050000,0.050000,0.050000") "Undefined" "OverrideRootScale" _characterref _characterref))
    (bind _output_get (Variables|Default|SetGrenadeRef _returnvalue))
    (Physics|SetSimulatePhysics (Variables|/Script/SoloLeveling.SL_HealthGrenade|GetMesh _output_get) false)
    (bind _returnvalue_2 (Transformation|AttachComponentToComponent _output_get (Variables|/Script/Engine.Character|GetMesh (Variables|Default|GetCharacterRef)) "hand_r" "SnapToTarget" "SnapToTarget" "KeepRelative" true))
    (Variables|Default|SetIsThrowing _returnvalue_2)
    (return _output_get)))

(fn UseGrenade
  (params (FollowCamera :type Camera%20Component%20Object%20Reference))
  (bind _grenaderef (Variables|Default|GetGrenadeRef)
    (:then
      (Transformation|DetachFromActor _grenaderef "KeepWorld" "KeepWorld" "KeepWorld")
      (Physics|SetSimulatePhysics (Variables|/Script/SoloLeveling.SL_HealthGrenade|GetMesh _grenaderef) true)
      (Class|SLHealthGrenade|UseGrenage _grenaderef (Math|Vector|GetForwardVector FollowCamera))
      (Variables|Default|SetGrenadeRef 0))
    (:else)))