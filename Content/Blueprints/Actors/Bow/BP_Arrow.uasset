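; BP_Arrow is an arrow projectile actor for the bow, launched through its Fire event with a direction and a strength.
; Fire adds a ProjectileMovement component at runtime, so the component does not exist until the shot.
; Strength interpolates launch speed from min to max and gravity scale from max to min, so stronger shots fly faster and flatter.
; A whoosh sound plays at the arrow's location on firing.
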(event Custom|Fire
  (params (Direction :type Vector) (Strength :type Float%20%28double-precision%29))
  (bind _returnvalue (AddComponent|AddProjectileMovementComponent))
  (Variables|/Script/Engine.MovementComponent|SetVelocity _returnvalue (* Direction (Math|Float|Lerp (Variables|Default|GetMinSpeed) (Variables|Default|GetMaxSpeed) Strength)))
  (Variables|/Script/Engine.ProjectileMovementComponent|SetProjectileGravityScale _returnvalue (Math|Float|Lerp (Variables|Default|GetMaxGravity) (Variables|Default|GetMinGravity) Strength))
  (Audio|PlaySoundatLocation (Variables|Default|GetWhoshSound) (Transformation|GetActorLocation) "0, 0, 0" 1.0 1.0 0.4 0 0 0 0))

(event EventBeginPlay)

(event Collision|EventActorBeginOverlap
  (params (OtherActor :type Actor%20Object%20Reference)))

(event EventTick
  (params (DeltaSeconds :type Float%20%28single-precision%29)))

(fn ConstructionScript)