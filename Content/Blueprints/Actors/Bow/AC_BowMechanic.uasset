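; Actor component that gives its owning Character a bow mechanic: equipping, aiming, drawing and firing arrows.
; BeginPlay spawns the bow onto a mesh socket; aiming switches movement to controller-facing rotation and attaches a new arrow.
; Drawing runs a looping timer whose accumulated time, normalized by the bow's max draw time, sets arrow strength along the camera's forward vector.
; A fire montage ends the shot and re-nocks an arrow if still aiming, while bow state follows each phase.
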(event Custom|AimBegin
  (bind _characterref (Variables|ObjectRefs|GetCharacterRef))
  (bind _charactermovement (Variables|/Script/Engine.Character|GetCharacterMovement _characterref))
  ;[0 0 0] Aim Bow
  (Variables|Booleans|SetIsAiming true)
  (Variables|/Script/Engine.CharacterMovementComponent|SetbOrientRotationToMovement _charactermovement false)
  (Variables|/Script/Engine.CharacterMovementComponent|SetbUseControllerDesiredRotation _charactermovement true)
  (Variables|/Script/Engine.CharacterMovementComponent|SetRotationRate _charactermovement (Variables|Default|GetAimRotationRate))
  (Variables|/Game/Blueprints/Actors/Bow/BP_Bow.BP_Bow_C|SetBowState (Variables|ObjectRefs|GetBowRef) "NewEnumerator1")
  (CallFunction|SpawnArrow))

(event Custom|AimEnd
  (bind _characterref (Variables|ObjectRefs|GetCharacterRef))
  (bind _charactermovement (Variables|/Script/Engine.Character|GetCharacterMovement _characterref))
  ;[0 0 0] Aim Bow
  (Variables|Booleans|SetIsAiming false)
  (CallFunction|DrawEnd)
  (Variables|/Script/Engine.CharacterMovementComponent|SetbOrientRotationToMovement _charactermovement true)
  (Variables|/Script/Engine.CharacterMovementComponent|SetbUseControllerDesiredRotation _charactermovement false)
  (Variables|/Script/Engine.CharacterMovementComponent|SetRotationRate _charactermovement (Variables|Default|GetInitialRotationRate))
  (Variables|/Game/Blueprints/Actors/Bow/BP_Bow.BP_Bow_C|SetBowState (Variables|ObjectRefs|GetBowRef) "NewEnumerator0")
  (CallFunction|DestroyArrow))

(event Custom|DrawBegin
  ;[0 0 0] Draw Bow
  (Utilities|CanDrawBow
    (:Yes
      (Variables|Booleans|SetIsDrawingBow true)
      (bind _returnvalue (Utilities|Time|SetTimerbyEvent (delegate Custom|IncrementDrawTime) (Variables|Default|GetDrawIncrementTime) true))
      (Variables|Default|SetDrawBowTimer _returnvalue)
      (Variables|/Game/Blueprints/Actors/Bow/BP_Bow.BP_Bow_C|SetBowState (Variables|ObjectRefs|GetBowRef) "NewEnumerator2"))))

(event Custom|DrawEnd
  ;[0 0 0] Draw Bow
  (Variables|Booleans|SetIsDrawingBow false)
  (Variables|Default|SetDrawTime 0.0)
  (Utilities|Time|ClearandInvalidateTimerbyHandle (Variables|Default|GetDrawBowTimer))
  (Variables|/Game/Blueprints/Actors/Bow/BP_Bow.BP_Bow_C|SetBowState (Variables|ObjectRefs|GetBowRef) "NewEnumerator0"))

(event Custom|IncrementDrawTime
  ;[0 0 0] Draw Bow
  (bind _output_get (Variables|Default|SetDrawTime (+ (Variables|Default|GetDrawTime) (Variables|Default|GetDrawIncrementTime))))
  (Development|PrintString (Utilities|String|ToString(Float) _output_get) true false "(R=0.422585,G=0.206690,B=1.000000,A=1.000000)" 0.0))

(event Custom|FireArrowBegin
  ;[0 0 0] Fire Arrow
  (if (Variables|Booleans|GetIsDrawingBow)
    (Variables|Booleans|SetIsFiringArrow true)
    (CallFunction|FireAimedArrow)
    (CallFunction|DrawEnd)
    (Animation|Montage|PlayMontage (Variables|/Script/Engine.Character|GetMesh (Variables|ObjectRefs|GetCharacterRef)) (Variables|Default|GetBowFireMontage)
      (:OnCompleted
        _)
      (:OnInterrupted
        _))
    (CallFunction|FireArrowEnd)))

(event Custom|FireArrowEnd
  ;[0 0 0] Fire Arrow
  (Variables|Booleans|SetIsFiringArrow false)
  (if (Variables|Booleans|GetIsAiming)
    (CallFunction|AimBegin)))

(event EventBeginPlay
  (bind _ascharacter (Utilities|Casting|CastToCharacter (Components|GetOwner)))
  (bind _output_get (Variables|ObjectRefs|SetCharacterRef _ascharacter))
  (CallFunction|EquipBow)
  (Variables|Default|SetInitialRotationRate (Variables|/Script/Engine.CharacterMovementComponent|GetRotationRate (Variables|/Script/Engine.Character|GetCharacterMovement _output_get))))

(fn EquipBow
  (bind _returnvalue (Game|SpawnActorfromClass (Variables|Classes|GetBowClass) (Math|Transform|MakeTransform "0, 0, 0" "0, 0, 0" "1.000000,1.000000,1.000000") "Undefined" "MultiplyWithRoot" 0 0))
  (bind _output_get (Variables|ObjectRefs|SetBowRef _returnvalue))
  (Transformation|AttachComponentToComponent _output_get (Variables|/Script/Engine.Character|GetMesh (Variables|ObjectRefs|GetCharacterRef)) (Variables|SocketNames|GetBowSocket) "SnapToTarget" "SnapToTarget" "SnapToTarget" true))

(fn SpawnArrow
  (bind _returnvalue (Game|SpawnActorfromClass (Variables|Classes|GetArrowClass) (Math|Transform|MakeTransform "0, 0, 0" "0, 0, 0" "1.000000,1.000000,1.000000") "Undefined" "MultiplyWithRoot" 0 0))
  (bind _output_get (Variables|ObjectRefs|SetArrowRef _returnvalue))
  (Transformation|AttachComponentToComponent _output_get (Variables|/Script/Engine.Character|GetMesh (Variables|ObjectRefs|GetCharacterRef)) (Variables|SocketNames|GetArrowSocketName) "SnapToTarget" "SnapToTarget" "SnapToTarget" true))

(fn DestroyArrow
  (bind _arrowref (Variables|ObjectRefs|GetArrowRef)
    (:then
      (Actor|DestroyActor _arrowref))
    (:else)))

(fn FireAimedArrow
  (bind _arrowref (Variables|ObjectRefs|GetArrowRef)
    (:then
      (Transformation|DetachFromActor _arrowref "KeepWorld" "KeepWorld" "KeepWorld")
      (Default|Fire _arrowref (Math|Vector|GetForwardVector (Actor|GetComponentbyClass (Variables|ObjectRefs|GetCharacterRef) "/Script/Engine.CameraComponent")) (Math|Float|Clamp(Float) (Math|Float|NormalizetoRange (Variables|Default|GetDrawTime) 0.0 (Variables|/Game/Blueprints/Actors/Bow/BP_Bow.BP_Bow_C|GetMaxDrawTIme (Variables|ObjectRefs|GetBowRef)))))
      (Variables|ObjectRefs|SetArrowRef 0))
    (:else)))