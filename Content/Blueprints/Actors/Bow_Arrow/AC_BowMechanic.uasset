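; Actor component that gives its owning Character a bow: it spawns and attaches the bow, then handles aiming, drawing and firing.
; Aiming switches movement to controller-facing rotation, sets bow state and spawns a socketed arrow, guarded by a delay timer.
; A looping timer accumulates draw time, broadcast through dispatchers and normalized into shot strength.
; After the fire montage, it re-aims if still aiming and resumes any queued draw.
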(event Custom|AimBegin
  (bind _characterref (Variables|ObjectRefs|GetCharacterRef))
  (bind _charactermovement (Variables|/Script/Engine.Character|GetCharacterMovement _characterref))
  ;[0 0 0] Aim Bow
  (if (Utilities|Time|IsTimerActivebyHandle (Variables|Default|GetAimDelayTimer))
    (Development|PrintString "Aim Timer Is Not Finished Yet" true true "(R=1.000000,G=0.000000,B=0.103125,A=1.000000)")
    (else
      (bind _returnvalue (Utilities|Time|SetTimerbyEvent (delegate Custom|AimDelayTimerFinish_Event) (Variables|Default|GetAimTimeDelay)))
      (bind _output_get (Variables|Default|SetAimDelayTimer _returnvalue))
      (if (Utilities|Time|IsTimerActivebyHandle _output_get)
        (Development|PrintString "Timer Is Started" true true "(R=1.000000,G=0.000000,B=0.103125,A=1.000000)")
        (Variables|Booleans|SetIsAiming true)
        (Variables|/Script/Engine.CharacterMovementComponent|SetbOrientRotationToMovement _charactermovement false)
        (Variables|/Script/Engine.CharacterMovementComponent|SetbUseControllerDesiredRotation _charactermovement true)
        (Variables|/Script/Engine.CharacterMovementComponent|SetRotationRate _charactermovement (Variables|Default|GetAimRotationRate))
        (Variables|/Game/Blueprints/Actors/Bow_Arrow/BP_Bow.BP_Bow_C|SetBowState (Variables|ObjectRefs|GetBowRef) "NewEnumerator1")
        (CallFunction|SpawnArrow)
        (Default|CallOnAimBegin)
        (else
          (Development|PrintString "Failed to Start the Timer" true true "(R=1.000000,G=0.000000,B=0.798588,A=1.000000)"))))))

(event Custom|AimEnd
  (bind _characterref (Variables|ObjectRefs|GetCharacterRef))
  (bind _charactermovement (Variables|/Script/Engine.Character|GetCharacterMovement _characterref))
  ;[0 0 0] Aim Bow
  (Variables|Booleans|SetIsAiming false)
  (CallFunction|DrawEnd)
  (Variables|/Script/Engine.CharacterMovementComponent|SetbOrientRotationToMovement _charactermovement true)
  (Variables|/Script/Engine.CharacterMovementComponent|SetbUseControllerDesiredRotation _charactermovement false)
  (Variables|/Script/Engine.CharacterMovementComponent|SetRotationRate _charactermovement (Variables|Default|GetInitialRotationRate))
  (Variables|/Game/Blueprints/Actors/Bow_Arrow/BP_Bow.BP_Bow_C|SetBowState (Variables|ObjectRefs|GetBowRef) "NewEnumerator0")
  (CallFunction|DestroyArrow)
  (Default|CallOnAimEnd)
  (Utilities|Time|ClearandInvalidateTimerbyHandle (Variables|Default|GetAimDelayTimer))
  (Development|PrintString "Aim Timer is Cleared" true true "(R=0.103635,G=1.000000,B=0.001999,A=1.000000)"))

(event Custom|DrawBegin
  ;[0 0 0] Draw Bow
  (Utilities|CanDrawBow
    (:Yes
      (Variables|Default|SetIsWaitingToDrawBow false)
      (Variables|Booleans|SetIsDrawingBow true)
      (bind _returnvalue (Utilities|Time|SetTimerbyEvent (delegate Custom|IncrementDrawTime) (Variables|Default|GetDrawIncrementTime) true))
      (Variables|Default|SetDrawBowTimer _returnvalue)
      (Default|DrawBegin (Variables|ObjectRefs|GetBowRef)))
    (:No
      ;;[0 0 0 0.5] Allows to Fire again while aiming
      (Variables|Default|SetIsWaitingToDrawBow true))))

(event Custom|DrawEnd
  ;[0 0 0] Draw Bow
  (Variables|Default|SetIsWaitingToDrawBow false)
  (Variables|Booleans|SetIsDrawingBow false)
  (Variables|Default|SetDrawTime 0.0)
  (Utilities|Time|ClearandInvalidateTimerbyHandle (Variables|Default|GetDrawBowTimer))
  (Default|DrawEnd (Variables|ObjectRefs|GetBowRef))
  (Default|CallOnDrawEnd))

(event Custom|IncrementDrawTime
  ;[0 0 0] Draw Bow
  (bind _output_get (Variables|Default|SetDrawTime (+ (Variables|Default|GetDrawTime) (Variables|Default|GetDrawIncrementTime))))
  (Development|PrintString (Utilities|String|ToString(Float) _output_get) true false "(R=0.422585,G=0.206690,B=1.000000,A=1.000000)" 0.0)
  (Default|CallOnDrawProgress (Variables|/Game/Blueprints/Actors/Bow_Arrow/BP_Bow.BP_Bow_C|GetMaxDrawTIme (Variables|ObjectRefs|GetBowRef)) _output_get))

(event Custom|FireArrowBegin
  (params (FireDirection :type Vector))
  ;[0 0 0] Fire Arrow
  (if (Variables|Booleans|GetIsDrawingBow)
    (Variables|Booleans|SetIsFiringArrow true)
    (CallFunction|FireAimedArrow FireDirection)
    (CallFunction|DrawEnd)
    (Animation|Montage|PlayMontage (Variables|/Script/Engine.Character|GetMesh (Variables|ObjectRefs|GetCharacterRef)) (Variables|Default|GetBowFireMontage)
      (:OnCompleted
        _)
      (:OnInterrupted
        _))
    (CallFunction|FireArrowEnd)))

(event Custom|FireArrowEnd
  ;[0 0 0] Fire Arrow
  (Variables|Booleans|SetIsFiringArrow false)
  (if (Variables|Booleans|GetIsAiming)
    (CallFunction|AimBegin)
    (Utilities|Time|ClearandInvalidateTimerbyHandle (Variables|Default|GetAimDelayTimer))
    (Development|PrintString "Aim Timer is Cleared" true true "(R=0.103635,G=1.000000,B=0.001999,A=1.000000)")
    (if (Variables|Default|GetIsWaitingToDrawBow)
      (CallFunction|DrawBegin))))

(event Custom|AimDelayTimerFinish_Event
  ;[0 0 0] Aim Bow
  (Development|PrintString "Aim Timer is finished" true true "(R=0.103635,G=1.000000,B=0.001999,A=1.000000)"))

(event EventBeginPlay
  ;[0 0 0 0.5] BeginPlay set Character Ref,  Rotation Rate, and Equip Bow function call
  (bind _ascharacter (Utilities|Casting|CastToCharacter (Components|GetOwner)))
  (bind _output_get (Variables|ObjectRefs|SetCharacterRef _ascharacter))
  (CallFunction|EquipBow)
  (Variables|Default|SetInitialRotationRate (Variables|/Script/Engine.CharacterMovementComponent|GetRotationRate (Variables|/Script/Engine.Character|GetCharacterMovement _output_get))))

(fn EquipBow
  (bind _returnvalue (Game|SpawnActorfromClass (Variables|Classes|GetBowClass) (Math|Transform|MakeTransform "0, 0, 0" "0, 0, 0" "1.000000,1.000000,1.000000") "Undefined" "MultiplyWithRoot" 0 0))
  (bind _output_get (Variables|ObjectRefs|SetBowRef _returnvalue))
  (Transformation|AttachComponentToComponent _output_get (Variables|/Script/Engine.Character|GetMesh (Variables|ObjectRefs|GetCharacterRef)) (Variables|SocketNames|GetBowSocket) "SnapToTarget" "SnapToTarget" "SnapToTarget" true))

(fn SpawnArrow
  (bind _returnvalue (Game|SpawnActorfromClass (Variables|Classes|GetArrowClass) (Math|Transform|MakeTransform "0, 0, 0" "0, 0, 0" "1.000000,1.000000,1.000000") "Undefined" "MultiplyWithRoot" 0 (Variables|ObjectRefs|GetCharacterRef)))
  (bind _output_get (Variables|ObjectRefs|SetArrowRef _returnvalue))
  (Transformation|AttachComponentToComponent _output_get (Variables|/Script/Engine.Character|GetMesh (Variables|ObjectRefs|GetCharacterRef)) (Variables|SocketNames|GetArrowSocketName) "SnapToTarget" "SnapToTarget" "SnapToTarget" true))

(fn DestroyArrow
  (bind _arrowref (Variables|ObjectRefs|GetArrowRef)
    (:then
      (Actor|DestroyActor _arrowref))
    (:else)))

(fn FireAimedArrow
  (params (FireDirection :type Vector))
  (bind _arrowref (Variables|ObjectRefs|GetArrowRef)
    (:then
      (Transformation|DetachFromActor _arrowref "KeepWorld" "KeepWorld" "KeepWorld")
      (Default|Fire _arrowref FireDirection (Math|Float|Clamp(Float) (Math|Float|NormalizetoRange (Variables|Default|GetDrawTime) 0.0 (Variables|/Game/Blueprints/Actors/Bow_Arrow/BP_Bow.BP_Bow_C|GetMaxDrawTIme (Variables|ObjectRefs|GetBowRef)))))
      (Variables|ObjectRefs|SetArrowRef 0))
    (:else)))