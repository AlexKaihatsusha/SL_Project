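; Bow arrow projectile that stays inert, with trail hidden and collision off, until Fire launches it.
; Fire adds a projectile movement component at runtime, scaling speed and gravity by draw strength, then enables trail and collision.
; Overlaps ignore the instigator; impacts stop and attach the arrow, play effects, push physics bodies and start a despawn timer.
; Arrows hitting each other are destroyed.
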(event OnComponentBeginOverlap(CollisionBox)
  (params (OverlappedComponent :type Primitive%20Component%20Object%20Reference) (OtherActor :type Actor%20Object%20Reference) (OtherComp :type Primitive%20Component%20Object%20Reference) (OtherBodyIndex :type Integer) (bFromSweep :type Boolean) (SweepResult :type Hit%20Result%20Structure%20%28by%20ref%29))
  (bind (_bblockinghit _binitialoverlap _time _distance _location _impactpoint _normal _impactnormal _physmat _hitactor _hitcomponent) (Collision|BreakHitResult SweepResult))
  (if (not (== OtherActor (Game|GetInstigator)))
    (bind _projectilemovementcomponent (Variables|Default|GetProjectileMovementComponent)
      (:then
        (Components|DestroyComponent _projectilemovementcomponent)
        (Collision|SetCollisionEnabled (Variables|Default|GetCollisionBox) "NoCollision")
        (if (!= _hitactor "BP_Arrow")
          (Transformation|AttachComponentToComponent _hitcomponent "None" "KeepWorld" "KeepWorld" "KeepWorld" true)
          (Audio|PlaySoundatLocation "/Game/Assets/SFX/Bow/arrow-impact-1.arrow-impact-1" (Transformation|GetActorLocation) "0, 0, 0" 1.0 1.0 0.0 0 0 0 0)
          (Actor|SetLifeSpan 5.0)
          (Niagara|SpawnSystematLocation (Variables|Default|GetImpactEffectSystem) _location (Math|Conversions|RotationFromXVector (- (Transformation|GetActorForwardVector) "")))
          (if (Physics|IsSimulatingPhysics _hitcomponent "None")
            (Physics|AddImpulse _hitcomponent (Variables|Default|GetArrowVelocity) "None" true))
          (else
            ;[0 0 0 0.5] Destoy both arrows if overlap with each other
            (Actor|DestroyActor)
            (Actor|DestroyActor))))
      (:else))))

(event Custom|Fire
  (params (Direction :type Vector) (Strength :type Float%20%28double-precision%29))
  (bind _returnvalue (AddComponent|AddProjectileMovementComponent))
  (Variables|Default|SetProjectileMovementComponent _returnvalue)
  (bind _output_get (Variables|/Script/Engine.MovementComponent|SetVelocity _returnvalue (* Direction (Math|Float|Lerp (Variables|Default|GetMinSpeed) (Variables|Default|GetMaxSpeed) Strength))))
  (Variables|Default|SetArrowVelocity _output_get)
  (Variables|/Script/Engine.ProjectileMovementComponent|SetProjectileGravityScale _returnvalue (Math|Float|Lerp (Variables|Default|GetMaxGravity) (Variables|Default|GetMinGravity) Strength))
  (Audio|PlaySoundatLocation (Variables|Default|GetWhoshSound) (Transformation|GetActorLocation) "0, 0, 0" 1.0 1.0 0.4 0 0 0 0)
  (Development|SetHiddeninGame (Variables|Default|GetNiagara_Trail) false false)
  (Collision|SetCollisionEnabled (Variables|Default|GetCollisionBox) "QueryAndPhysics"))

(event EventBeginPlay
  ;[0 0 0 0.5] Hide the Trail
  (Development|SetHiddeninGame (Variables|Default|GetNiagara_Trail) true false)
  (Collision|SetCollisionEnabled (Variables|Default|GetCollisionBox) "NoCollision"))

(event Collision|EventActorBeginOverlap
  (params (OtherActor :type Actor%20Object%20Reference)))

(event EventTick
  (params (DeltaSeconds :type Float%20%28single-precision%29)))

(fn ConstructionScript)