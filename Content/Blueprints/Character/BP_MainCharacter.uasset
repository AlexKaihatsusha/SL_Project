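; BP_MainCharacter is the player character Blueprint, handling bow aiming and grenade throwing.
; The bow input starts and ends aiming on ACBowMechanic, while a timeline played forward and reversed blends camera FOV and boom socket offset from values cached at BeginPlay.
; The throw input spawns a BP_HealthGrenade offset along world X from the character and immediately uses it.
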(event Custom|AimCameraEnd
  (bind _aimalpha (Timeline|AimCameraTimeLine Reverse)
    (:Update
      (Camera|SetFieldOfView (Variables|Default|GetFollowCamera) (Math|Float|Lerp (Variables|Default|GetInitial%20FOV) (Variables|Default|GetAim%20FOV) _aimalpha))
      (Variables|/Script/Engine.SpringArmComponent|SetSocketOffset (Variables|Default|GetCameraBoom) (Math|Vector|Lerp(Vector) (Variables|Default|GetInitialBoomOffset) (Variables|Default|GetAimBoomOffset) _aimalpha)))))

(event Custom|AimCameraBegin
  (bind _aimalpha (Timeline|AimCameraTimeLine Play)
    (:Update
      (Camera|SetFieldOfView (Variables|Default|GetFollowCamera) (Math|Float|Lerp (Variables|Default|GetInitial%20FOV) (Variables|Default|GetAim%20FOV) _aimalpha))
      (Variables|/Script/Engine.SpringArmComponent|SetSocketOffset (Variables|Default|GetCameraBoom) (Math|Vector|Lerp(Vector) (Variables|Default|GetInitialBoomOffset) (Variables|Default|GetAimBoomOffset) _aimalpha)))))

(event Input|EnhancedActionEvents|EnhancedInputActionIA_Throw
  (params (ActionValue :type Boolean) (ElapsedSeconds :type Float%20%28double-precision%29) (TriggeredSeconds :type Float%20%28double-precision%29) (InputAction :type Input%20Action%20Object%20Reference :default "/Game/Blueprints/Character/Input/Actions/IA_Throw.IA_Throw"))
  (bind _returnvalue (Transformation|GetActorTransform))
  (bind _returnvalue_2 (Game|SpawnActorfromClass "/Game/Blueprints/Actors/Grenade/BP_HealthGrenade.BP_HealthGrenade_C" (Math|Transform|MakeTransform (Math|Vector|MakeVector (+ (.x (.location _returnvalue)) 1e+02) (.y (.location _returnvalue)) (.z (.location _returnvalue))) (.rotation _returnvalue) (.scale _returnvalue)) "AdjustIfPossibleButAlwaysSpawn" "MultiplyWithRoot" 0 self))
  (Class|SLHealthGrenade|UseGrenage _returnvalue_2))

(event Input|EnhancedActionEvents|EnhancedInputActionIA_Bow
  (params (ActionValue :type Boolean) (ElapsedSeconds :type Float%20%28double-precision%29) (TriggeredSeconds :type Float%20%28double-precision%29) (InputAction :type Input%20Action%20Object%20Reference :default "/Game/Blueprints/Character/Input/Actions/IA_Bow.IA_Bow"))
  (:Started
    (Default|AimBegin (Variables|Default|GetAC_BowMechanic))
    (CallFunction|AimCameraBegin))
  (:Completed
    (Default|AimEnd (Variables|Default|GetAC_BowMechanic))
    (CallFunction|AimCameraEnd)))

(event EventBeginPlay
  (Variables|Default|SetInitial%20FOV (Variables|/Script/Engine.CameraComponent|GetFieldOfView (Variables|Default|GetFollowCamera)))
  (Variables|Default|SetInitialBoomOffset (Variables|/Script/Engine.SpringArmComponent|GetSocketOffset (Variables|Default|GetCameraBoom))))

(event Collision|EventActorBeginOverlap
  (params (OtherActor :type Actor%20Object%20Reference)))

(event EventTick
  (params (DeltaSeconds :type Float%20%28single-precision%29)))

(fn ConstructionScript)