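; Player character that aims and fires a bow, throws grenades and creates the HUD on BeginPlay.
; Input is forwarded to the bow and grenade components, with throws blocked while aiming or already throwing.
; A timeline blends camera FOV and boom offset for aiming, while a camera trace gives the direction from arrow to target point.
; Death, block and damage events only print placeholders, and an enemy-state test toggle is unwired.
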(event Custom|CreateHUD
  ;[0 0 0 0.5] Create HUD
  (bind _returnvalue (UserInterface|CreateWidget "/Game/Blueprints/Widgets/Bow/WBP_HUD.WBP_HUD_C"))
  (bind _output_get (Variables|Default|SetHUDRef _returnvalue))
  (UserInterface|Viewport|AddtoViewport _output_get 0))

(event Custom|AimCameraEnd
  ;[0 0 0 0.5] Aim Camera
  (bind _aimalpha (Timeline|AimCameraTimeLine Reverse)
    (:Update
      (Camera|SetFieldOfView (Variables|Default|GetFollowCamera) (Math|Float|Lerp (Variables|Default|GetInitial%20FOV) (Variables|Default|GetAim%20FOV) _aimalpha))
      (Variables|/Script/Engine.SpringArmComponent|SetSocketOffset (Variables|Default|GetCameraBoom) (Math|Vector|Lerp(Vector) (Variables|Default|GetInitialBoomOffset) (Variables|Default|GetAimBoomOffset) _aimalpha)))))

(event Custom|AimCameraBegin
  ;[0 0 0 0.5] Aim Camera
  (bind _aimalpha (Timeline|AimCameraTimeLine Play)
    (:Update
      (Camera|SetFieldOfView (Variables|Default|GetFollowCamera) (Math|Float|Lerp (Variables|Default|GetInitial%20FOV) (Variables|Default|GetAim%20FOV) _aimalpha))
      (Variables|/Script/Engine.SpringArmComponent|SetSocketOffset (Variables|Default|GetCameraBoom) (Math|Vector|Lerp(Vector) (Variables|Default|GetInitialBoomOffset) (Variables|Default|GetAimBoomOffset) _aimalpha)))))

(event Custom|InitVariables
  (Variables|Default|SetInitial%20FOV (Variables|/Script/Engine.CameraComponent|GetFieldOfView (Variables|Default|GetFollowCamera)))
  (Variables|Default|SetInitialBoomOffset (Variables|/Script/Engine.SpringArmComponent|GetSocketOffset (Variables|Default|GetCameraBoom))))

(event Custom|Dead
  (Development|PrintString "DEAD"))

(event Custom|DamageEffect
  (params (DamageEffect :type Byte :default 0))
  (Development|PrintString "Hello"))

(event Custom|Blocked
  (params (CanBeParried :type Boolean))
  (Development|PrintString "BLOCKED"))

(event Input|EnhancedActionEvents|EnhancedInputActionIA_Throw
  (params (ActionValue :type Boolean) (ElapsedSeconds :type Float%20%28double-precision%29) (TriggeredSeconds :type Float%20%28double-precision%29) (InputAction :type Input%20Action%20Object%20Reference :default "/Game/Blueprints/Player/Input/Actions/IA_Throw.IA_Throw"))
  (bind _ac_grenademechanic (Variables|Default|GetAC_GrenadeMechanic))
  ;[0 0 0 0.5] Throw Grenade
  (if (and (not (Variables|/Game/Blueprints/DamageActors/Bow_Arrow/AC_BowMechanic.AC_BowMechanic_C|GetIsAiming (Variables|Default|GetAC_BowMechanic))) (not (Variables|/Game/Blueprints/DamageActors/Grenade/AC_GrenadeMechanic.AC_GrenadeMechanic_C|GetIsThrowing _ac_grenademechanic)))
    (Default|ThrowGrenade _ac_grenademechanic (Variables|Default|GetFollowCamera))))

(event Input|EnhancedActionEvents|EnhancedInputActionIA_Bow
  (params (ActionValue :type Boolean) (ElapsedSeconds :type Float%20%28double-precision%29) (TriggeredSeconds :type Float%20%28double-precision%29) (InputAction :type Input%20Action%20Object%20Reference :default "/Game/Blueprints/Player/Input/Actions/IA_Bow.IA_Bow"))
  ;[0 0 0 0.5] Bow Input
  (:Started
    (Default|AimBegin (Variables|Default|GetAC_BowMechanic))
    (CallFunction|AimCameraBegin))
  (:Completed
    (Default|AimEnd (Variables|Default|GetAC_BowMechanic))
    (CallFunction|AimCameraEnd)))

(event Input|EnhancedActionEvents|EnhancedInputActionIA_BowFire
  (params (ActionValue :type Boolean) (ElapsedSeconds :type Float%20%28double-precision%29) (TriggeredSeconds :type Float%20%28double-precision%29) (InputAction :type Input%20Action%20Object%20Reference :default "/Game/Blueprints/Player/Input/Actions/IA_BowFire.IA_BowFire"))
  (bind _ac_bowmechanic (Variables|Default|GetAC_BowMechanic))
  ;[0 0 0 0.5] Bow Input
  (:Started
    (Default|DrawBegin _ac_bowmechanic))
  (:Completed
    (bind _direction (CallFunction|CalculateAimDirection))
    (Default|FireArrowBegin _ac_bowmechanic _direction)))

(event EventBeginPlay
  (CallFunction|InitVariables)
  (CallFunction|CreateHUD))

(event Input|KeyboardEvents|1
  (params (Key :type Key%20Structure :default "None")))

(fn ConstructionScript)

(fn CalculateAimDirection
  (bind _followcamera (Variables|Default|GetFollowCamera))
  (bind _returnvalue (Transformation|GetWorldLocation _followcamera))
  ;[0 0 0 0.5] Use Line Trace By Channel to Set a Direction(to hit location or trace end location) to Arrow Projectile
  (bind (_outhit _returnvalue_2) (Collision|LineTraceByChannel _returnvalue (+ (* (Math|Vector|GetForwardVector _followcamera) 1e+04) _returnvalue) "TraceTypeQuery1" false 0 "None"))
  (bind _arrowref (Variables|/Game/Blueprints/DamageActors/Bow_Arrow/AC_BowMechanic.AC_BowMechanic_C|GetArrowRef (Variables|Default|GetAC_BowMechanic))
    (:then
      (return (Math|Vector|GetUnitDirection(Vector) (Transformation|GetActorLocation _arrowref) (Math|Vector|SelectVector (.Location (Collision|BreakHitResult _outhit)) (.TraceEnd (Collision|BreakHitResult _outhit)) _returnvalue_2))))
    (:else)))